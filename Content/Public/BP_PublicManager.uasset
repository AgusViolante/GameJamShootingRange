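; BP_PublicManager is an actor that fills a stand with crowd members and makes them cheer.
; On BeginPlay it spawns BP_Public actors in a row-and-column grid from its location, with random horizontal jitter and each row raised higher like bleachers.
; It stores the spawned actors in PublicArray, and its Cheers event relays the call to each one.
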(event `self.ReceiveBeginPlay`
  (bind (_returnvalue_x _returnvalue_y) (`KismetMathLibrary.BreakVector` (`self.K2_GetActorLocation`)))
  (bind _returnvalue_x_2 (`KismetMathLibrary.BreakVector` (`self.K2_GetActorLocation`)))
  (bind (_returnvalue_x_3 _returnvalue_y_2 _returnvalue_z) (`KismetMathLibrary.BreakVector` (`self.K2_GetActorLocation`)))
  (for _index (range (+ (`self.MaxRows`) 1))
    (for _index_2 (range (+ (`self.MaxColumns`) 1))
      (bind _returnvalue (`|SpawnActorFromClass` "/Game/Public/BP_Public.BP_Public_C" (`KismetMathLibrary.MakeTransform` (`KismetMathLibrary.MakeVector` (+ (+ (* _index 300.0) _returnvalue_x_2) (`KismetMathLibrary.RandomFloatInRange` -30.0 30.0)) (+ (+ (* _index_2 150.0) _returnvalue_y) (`KismetMathLibrary.RandomFloatInRange` -30.0 30.0)) (+ (* _index 25.0) _returnvalue_z)) (`self.K2_GetActorRotation`)) "Undefined" "MultiplyWithRoot" null null))
      (`KismetArrayLibrary.Array_AddUnique` (`self.PublicArray`) _returnvalue))))

(event `Cheers`
  (for _array_element (`self.PublicArray`)
    (`/Game/Public/BP_Public.Cheers` _array_element)))

(fn `UserConstructionScript`)