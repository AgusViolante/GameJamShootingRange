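; BP_Public is an audience member represented by a plane that bobs up and down and can cheer.
; BeginPlay randomizes the plane's width and height, then loops on random delays with a weighted chance of an idle move.
; RandomMove and Cheers each drive a timeline that lerps the plane's relative Z location.
; Cheers adds a short random delay to stagger reactions, and nothing live in this Blueprint calls it.
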(event `self.ReceiveBeginPlay`
  (`SceneComponent.SetRelativeScale3D` (`self.Plane`) (`KismetMathLibrary.MakeVector` (`KismetMathLibrary.RandomFloatInRange` 1.0 1.0) (`KismetMathLibrary.RandomFloatInRange` 1.0 1.5) (`KismetMathLibrary.RandomFloatInRange` 1.0 4.1)))
  (`KismetSystemLibrary.Delay` (`KismetMathLibrary.RandomFloatInRange` 5.0 25.0) :!label _label)
  (if (`KismetMathLibrary.RandomBoolWithWeight` 0.3)
    (`self.RandomMove`)
    (goto _label)
    (else
      (goto _label))))

(event `RandomMove`
  (bind (_direction _lerp) (`Timeline|Move` :!via `PlayFromStart`)
    (:`Update`
      (`SceneComponent.K2_SetRelativeLocation` (`self.Plane`) (`KismetMathLibrary.MakeVector` 0.0 0.0 (`KismetMathLibrary.Lerp` 50.0 65.0 _lerp)) false false))))

(event `Cheers`
  (`KismetSystemLibrary.Delay` (`KismetMathLibrary.RandomFloatInRange` 0.0 0.2))
  (bind (_direction _lerp) (`Timeline|Timeline` :!via `PlayFromStart`)
    (:`Update`
      (`SceneComponent.K2_SetRelativeLocation` (`self.Plane`) (`KismetMathLibrary.MakeVector` 0.0 0.0 (`KismetMathLibrary.Lerp` 50.0 65.0 _lerp)) false false))))

(fn `UserConstructionScript`)