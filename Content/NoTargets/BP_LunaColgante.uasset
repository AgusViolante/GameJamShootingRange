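; Hanging moon actor that bobs its Pendulo component up and down like an elevator, starting at BeginPlay after the parent's own setup runs.
; The SubeBaja timeline drives a Lerp on the component's relative Z between two fixed heights, leaving X and Y unchanged.
; ElevatorMoon flips the IsForwar flag to play or reverse the timeline, and its Finished output calls the event again for an endless ping-pong loop.
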(event `self.ReceiveBeginPlay`
  (`parent.ReceiveBeginPlay`)
  (`self.ElevatorMoon`))

(event `ElevatorMoon`
  (bind _pendulo (`self.Pendulo`))
  (bind (_relativelocation_x _relativelocation_y) (`KismetMathLibrary.BreakVector` (`SceneComponent.RelativeLocation` _pendulo)))
  (if (`self.IsForwar`)
    (set `self.IsForwar` false)
    (bind (_direction _alpha) (`Timeline|SubeBaja` :!label _label)
      (:`Update`
        (`SceneComponent.K2_SetRelativeLocation` _pendulo (`KismetMathLibrary.MakeVector` _relativelocation_x _relativelocation_y (`KismetMathLibrary.Lerp` 1200.0 350.0 _alpha)) false false))
      (:`Finished`
        (`self.ElevatorMoon`)))
    (else
      (set `self.IsForwar` true)
      (goto _label :!via `Reverse`))))

(fn `UserConstructionScript`
  (`parent.UserConstructionScript`))