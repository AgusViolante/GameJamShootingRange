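; BP_PenduloNube1 is a cloud pendulum, judging by its name, that swings continuously back and forth once play begins.
; BeginPlay sets opposite pitch limits, then RotationReset alternately plays and reverses the Pendulo_TL timeline by toggling IsForward.
; The timeline alpha lerps the Pendulo component's relative pitch, and its Finished output calls RotationReset again to loop.
; The MoveTarget event is present but empty.
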(event `self.ReceiveBeginPlay`
  (`parent.ReceiveBeginPlay`)
  (`|ExecutionSequence`
    (:`then_0`
      (set `self.StartRotationY` 65.0)
      (set `self.EndRotationY` -65.0))
    (:`then_1`
      (`self.RotationReset`))))

(event `RotationReset`
  (if (`self.IsForward`)
    (set `self.IsForward` false)
    (bind (_direction _alpha) (`Timeline|Pendulo_TL` :!label _label)
      (:`Update`
        (`SceneComponent.K2_SetRelativeRotation` (`self.Pendulo`) (`KismetMathLibrary.MakeRotator` 0.0 (`KismetMathLibrary.Lerp` (`self.StartRotationY`) (`self.EndRotationY`) _alpha)) false false))
      (:`Finished`
        (`self.RotationReset`)))
    (else
      (set `self.IsForward` true)
      (goto _label :!via `Reverse`))))

(event `self.MoveTarget`)

(fn `UserConstructionScript`
  (`parent.UserConstructionScript`))