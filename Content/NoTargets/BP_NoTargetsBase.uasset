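; BP_NoTargetsBase is a base Blueprint for a "no target" object that moves back and forth between its start position and an end point.
; BeginPlay caches both relative locations and starts MoveTarget.
; A timeline lerps the NoTarget component between them at MoveRate.
; On each finish MoveTarget runs again, flipping IsForward to alternate Play and Reverse for an endless ping-pong.
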(event `self.ReceiveBeginPlay`
  (set `self.StartingLocation` (`SceneComponent.RelativeLocation` (`self.NoTarget`)))
  (set `self.EndLocation` (`SceneComponent.RelativeLocation` (`self.EndPoint`)))
  (`self.MoveTarget`))

(event `MoveTarget`
  (`TimelineComponent.SetPlayRate` (`self.Move_NoTarget`) (`self.MoveRate`))
  (if (`self.IsForward`)
    (set `self.IsForward` false)
    (bind (_direction _alpha) (`Timeline|Move_NoTarget` :!label _label)
      (:`Update`
        (`SceneComponent.K2_SetRelativeLocation` (`self.NoTarget`) (`KismetMathLibrary.VLerp` (`self.StartingLocation`) (`self.EndLocation`) _alpha) false false))
      (:`Finished`
        (`self.MoveTarget`)))
    (else
      (set `self.IsForward` true)
      (goto _label :!via `Reverse`))))

(fn `UserConstructionScript`)