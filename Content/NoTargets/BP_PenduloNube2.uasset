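; Pendulum cloud actor that rotates its Pendulo component in pitch through a timeline-driven swing.
; BeginPlay sets symmetric start and end angles, then calls RotationReset, which plays or reverses Pendulo_TL according to IsForward.
; The timeline's Alpha interpolates the pitch, and its Finished pin calls RotationReset again.
; Both branches write IsForward back to the value just tested, so the direction never toggles here.
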(event `self.ReceiveBeginPlay`
  (`parent.ReceiveBeginPlay`)
  (`|ExecutionSequence`
    (:`then_0`
      (set `self.StartRotationY` 65.0)
      (set `self.EndRotationY` -65.0))
    (:`then_1`
      (`self.RotationReset`))))

(event `RotationReset`
  (if (`self.IsForward`)
    (set `self.IsForward` true)
    (bind (_direction _alpha) (`Timeline|Pendulo_TL` :!label _label)
      (:`Update`
        (`SceneComponent.K2_SetRelativeRotation` (`self.Pendulo`) (`KismetMathLibrary.MakeRotator` 0.0 (`KismetMathLibrary.Lerp` (`self.StartRotationY`) (`self.EndRotationY`) _alpha)) false false))
      (:`Finished`
        (`self.RotationReset`)))
    (else
      (set `self.IsForward` false)
      (goto _label :!via `Reverse`))))

(fn `UserConstructionScript`
  (`parent.UserConstructionScript`))