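; BP_FinalBoss is the final boss enemy, handling a timed entrance triggered by the shooter game mode's OnStart event.
; It binds to that event on BeginPlay, waits 55 seconds after it fires, then reveals the Mask2003 component.
; A timeline lowers the mask along Z and, on finishing, calls SetMultiplier on the player's BP_ShooterCharacter.
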(event `self.ReceiveBeginPlay`
  (bind _asbp_shooter_game_mode (cast `/Game/Variant_Shooter/Blueprints/BP_ShooterGameMode` (`GameplayStatics.GetGameMode`)))
  (add `/Game/Variant_Shooter/Blueprints/BP_ShooterGameMode.OnStart` _asbp_shooter_game_mode (delegate `OnStart_Event`)))

(event `OnStart_Event`
  (bind _mask2_003 (`self.Mask2_003`))
  (bind (_relativelocation_x _relativelocation_y) (`KismetMathLibrary.BreakVector` (`SceneComponent.RelativeLocation` _mask2_003)))
  (`KismetSystemLibrary.Delay` 55.0)
  (`SceneComponent.SetVisibility` (`self.Mask2_003`) true false)
  (bind (_direction _lerp) (`Timeline|Timeline` :!via `PlayFromStart`)
    (:`Update`
      (`SceneComponent.K2_SetRelativeLocation` _mask2_003 (`KismetMathLibrary.MakeVector` _relativelocation_x _relativelocation_y (`KismetMathLibrary.Lerp` 1220.0 526.0 _lerp)) false false))
    (:`Finished`
      (bind _asbp_shooter_character (cast `/Game/Variant_Shooter/Blueprints/BP_ShooterCharacter` (`GameplayStatics.GetPlayerPawn` 0)))
      (`/Game/Variant_Shooter/Blueprints/BP_ShooterCharacter.SetMultiplier` _asbp_shooter_character))))

(fn `UserConstructionScript`)