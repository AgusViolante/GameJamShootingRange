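; BP_EnemyMask1 is an enemy mask actor that appears with a random look and can visually break.
; On BeginPlay it runs the parent logic, sets its static mesh to a random pick from RandomMask and plays an attenuated spawn sound.
; The SpawnMaskVFX event spawns the Niagara break effect at the mesh's transform, hides the mesh and plays a hit sound, without destroying the actor.
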(event `self.ReceiveBeginPlay`
  (`parent.ReceiveBeginPlay`)
  (`StaticMeshComponent.SetStaticMesh` (`self.StaticMesh`) (`KismetArrayLibrary.Array_Random` (`self.RandomMask`)))
  (`GameplayStatics.PlaySoundAtLocation` "/Game/SFXs/Spawn_Mask_V1.Spawn_Mask_V1" (`self.K2_GetActorLocation`) (struct) 1.0 1.0 0.0 "/Game/SFXs/Attenuation.Attenuation" null null null))

(event `self.SpawnMaskVFX`
  (bind _staticmesh (`self.StaticMesh`))
  (`NiagaraFunctionLibrary.SpawnSystemAtLocation` "/Game/Enemies/NS_MaskBreak.NS_MaskBreak" (`SceneComponent.K2_GetComponentLocation` _staticmesh) (`SceneComponent.K2_GetComponentRotation` _staticmesh))
  (`SceneComponent.SetVisibility` _staticmesh false false)
  (`GameplayStatics.PlaySoundAtLocation` "/Game/SFXs/Hit_Mascara__exito_.Hit_Mascara__exito_" (`self.K2_GetActorLocation`) (struct) 1.0 1.0 0.0 "/Game/SFXs/Attenuation.Attenuation" null null null))

(fn `UserConstructionScript`
  (`parent.UserConstructionScript`))