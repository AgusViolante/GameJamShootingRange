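; BP_EnemyAA is a moving shooting-range target that awards the player a point when damaged.
; BeginPlay waits briefly, raises the target if down, and gives InterpToMovement a relative path to MovementOffset.
; Timelines lerp the Sphere's rotation for raise and drop, gated by IsDown.
; Damage calls UpdateScore on BP_ShooterCharacter, plays the drop, then destroys the actor after a delay.
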(event `self.ReceiveTick`
  (params (DeltaSeconds :type "Float (single-precision)")))

(event `self.ReceiveAnyDamage`
  (params (Damage :type "Float (single-precision)") (DamageType :type "DamageType Object Reference") (InstigatedBy :type "Controller Object Reference") (DamageCauser :type "Actor Object Reference"))
  (`self.UpdateScore` 1)
  (`self.PlayTargetDrop`)
  (`KismetSystemLibrary.Delay` 1.0)
  (`self.K2_DestroyActor`))

(event `self.ReceiveBeginPlay`
  (set `self.Relative Rotation REf` (`SceneComponent.RelativeRotation` (`self.Sphere`)))
  (`KismetSystemLibrary.Delay` 2.0)
  (`self.RaiseEnem`)
  (`self.LineMovement`))

(event `PlayTargetDrop`
  (if (not (`self.IsDown?`))
    (set `self.IsDown?` true)
    (bind (_direction _alpha) (`Timeline|DropTarget`)
      (:`Update`
        (`SceneComponent.K2_SetRelativeRotation` (`self.Sphere`) (`KismetMathLibrary.RLerp` (`self.Relative Rotation REf`) (struct :`Pitch` 90.0) _alpha) false false)))))

(event `RaiseEnem`
  (if (`self.IsDown?`)
    (set `self.IsDown?` false)
    (bind (_direction _alpha2) (`Timeline|RaiseTarget`)
      (:`Update`
        (`SceneComponent.K2_SetRelativeRotation` (`self.Sphere`) (`KismetMathLibrary.RLerp` (`self.Relative Rotation REf`) (struct) _alpha2) false false)
        (set `self.Relative Rotation REf` (struct))))))

(event `LineMovement`
  (bind _interptomovement (`self.InterpToMovement`))
  (`InterpToMovementComponent.AddControlPointPosition` _interptomovement (0.0 0.0 0.0) true)
  (`InterpToMovementComponent.AddControlPointPosition` _interptomovement (`self.MovementOffset`) true)
  (`InterpToMovementComponent.FinaliseControlPoints` _interptomovement))

(fn `UpdateScore`
  (params (Score :type Integer))
  (bind _asbp_shooter_character (cast `/Game/Variant_Shooter/Blueprints/BP_ShooterCharacter` (`GameplayStatics.GetPlayerPawn` 0)))
  (`/Game/Variant_Shooter/Blueprints/BP_ShooterCharacter.UpdateScore` _asbp_shooter_character Score))

(fn `UserConstructionScript`)