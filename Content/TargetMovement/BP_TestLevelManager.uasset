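; Test level manager that runs a timed sequence of target spawns and fades in a music track when the shooter game mode fires OnStart.
; SpawnNextEnemy re-calls itself through CurrentWaveConfig's enemy list, delaying each spawn and passing its movement offset, data and index to the target.
; A hard-coded index triggers BeginFinalBoss, which is still empty.
; Unwired nodes hold start indices for skipping to later waves.
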(event `self.ReceiveBeginPlay`
  (bind _asbp_shooter_game_mode (cast `/Game/Variant_Shooter/Blueprints/BP_ShooterGameMode` (`GameplayStatics.GetGameMode`)))
  (add `/Game/Variant_Shooter/Blueprints/BP_ShooterGameMode.OnStart` _asbp_shooter_game_mode (delegate `OnStart_Event`)))

(event `OnStart_Event`
  (`self.Start Wave`)
  (`AudioComponent.FadeIn` (`self.Opera_V1__BORRADOR_`) 0.3 1.0 0.0 "Linear"))

(event `Start Wave`
  (set `self.CurrentIndex` 0)
  (`self.Spawn Next Enemy`))

(event `Spawn Next Enemy`
  (bind _currentindex (`self.CurrentIndex`))
  (bind _currentindex_2 (`self.CurrentIndex`))
  (bind _enemylist (`/Game/TargetMovement/BP_WaveConfig.EnemyList` (`self.CurrentWaveConfig`)))
  (bind (_output_targetclass _output_spawnlocation _output_waittime _output_movevector) (break `/Game/TargetMovement/S_SpawnInfo` (`|GetArrayItem` _enemylist _currentindex_2)))
  (if (< _currentindex (`KismetArrayLibrary.Array_Length` _enemylist))
    (`KismetSystemLibrary.Delay` _output_waittime)
    (`|SpawnActorFromClass` _output_targetclass (`KismetMathLibrary.MakeTransform` _output_spawnlocation) "AlwaysSpawn" "MultiplyWithRoot" null _output_movevector (`|GetArrayItem` _enemylist _currentindex_2) _currentindex null)
    (`/Engine/EditorBlueprintResources/StandardMacros.IncrementInt` (`self.CurrentIndex`)
      (:`  `
        (`self.Spawn Next Enemy`)
        (if (== (`self.CurrentIndex`) 57)
          (`self.BeginFinalBoss`))))))

(event `BeginFinalBoss`)

(fn `UserConstructionScript`)